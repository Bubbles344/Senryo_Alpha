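; BP_Anvil is an anvil hazard that marks the ground beneath it and splats on impact.
; On BeginPlay it traces straight down, spawns a shadow effect at that point and disables Hitbox1 collision.
; Its first Hit spawns a splat effect at the cached trace point, enables Hitbox1, then destroys the anvil after a short delay.
; The overlapping-actor loop is empty, and the Squash and TakeDamage calls are unconnected.
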(event Collision|EventActorBeginOverlap
  (params (OtherActor :type Actor%20Object%20Reference)))

(event EventTick
  (params (DeltaSeconds :type Float%20%28single-precision%29)))

(event Collision|EventHit
  (params (MyComp :type Primitive%20Component%20Object%20Reference) (Other :type Actor%20Object%20Reference) (OtherComp :type Primitive%20Component%20Object%20Reference) (bSelfMoved :type Boolean) (HitLocation :type Vector :default "0, 0, 0") (HitNormal :type Vector :default "0, 0, 0") (NormalImpulse :type Vector :default "0, 0, 0") (Hit :type Hit%20Result%20Structure%20%28by%20ref%29))
  (Utilities|FlowControl|DoOnce false
    (:Completed
      (for _index (range 0 (Utilities|Array|Length (Collision|GetOverlappingActors (Variables|Default|Gethitbox) 0 :!class /Script/Engine.PrimitiveComponent)))
        _)
      (Niagara|SpawnSystematLocation "/Game/VFX/AnvilSplat.AnvilSplat" (+ (.location (stale EventBeginPlay _outhit)) "0, 0,10.000000"))
      (Collision|SetCollisionEnabled (Variables|Default|Gethitbox1) "QueryAndPhysics")
      (Utilities|FlowControl|Delay 2.0)
      (Actor|DestroyActor))))

(event EventBeginPlay
  (bind _returnvalue (Transformation|GetActorLocation))
  (bind _returnvalue_2 (+ _returnvalue "0,-10.000000, 0"))
  (bind _outhit (Collision|LineTraceByChannel _returnvalue_2 (- _returnvalue_2 (Math|Vector|MakeVector 0.0 0.0 1e+04)) "TraceTypeQuery1" false 0 "None"))
  (Niagara|SpawnSystematLocation "/Game/VFX/AnvilShadow2.AnvilShadow2" (+ (.location _outhit) "0, 0,10.000000"))
  (Collision|SetCollisionEnabled (Variables|Default|Gethitbox1) "NoCollision"))

(fn ConstructionScript)