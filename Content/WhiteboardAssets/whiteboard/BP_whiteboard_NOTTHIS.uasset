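; Whiteboard actor that lets the player draw on its surface with the mouse.
; On BeginPlay it enables input, creates a dynamic sharpie material and clears the render target.
; While left mouse is held, Tick traces complex collision under the cursor and passes the hit UV to the hit whiteboard.
; DrawOnWhiteboard sets that UV as the material's draw location and draws the material into the render target.
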(event Custom|DrawOnWhiteboard
  (params (locationtodraw :type Vector%202D%20Structure))
  (bind _sharpieinstance (Variables|Default|GetSharpieInstance))
  (Rendering|Material|SetVectorParameterValue _sharpieinstance "drawLocation" (Math|Conversions|ToLinearColor(Vector) (Math|Conversions|ToVector(Vector2D) locationtodraw)) :!class /Script/Engine.MaterialInstanceDynamic)
  (Rendering|DrawMaterialtoRenderTarget "/Game/WhiteboardAssets/whiteboard/RT_WHITEBOARD_NOTTHIS.RT_WHITEBOARD_NOTTHIS" _sharpieinstance))

(event EventBeginPlay
  (Input|EnableInput (Game|GetPlayerController 0))
  (bind _returnvalue (Rendering|Material|CreateDynamicMaterialInstance "/Game/WhiteboardAssets/whiteboard/M_sharpie_NOTTHIS.M_sharpie_NOTTHIS" "None" "None" :!class /Script/Engine.KismetMaterialLibrary))
  (Variables|Default|SetSharpieInstance _returnvalue)
  (Rendering|ClearRenderTarget2D "/Game/WhiteboardAssets/whiteboard/RT_WHITEBOARD_NOTTHIS.RT_WHITEBOARD_NOTTHIS"))

(event EventTick
  (params (DeltaSeconds :type Float%20%28single-precision%29))
  (bind _returnvalue (Game|GetPlayerController 0))
  (bind (_worldlocation _worlddirection) (Game|Player|ConvertMouseLocationToWorldSpace _returnvalue))
  (if (Variables|Default|GetMousepressed%20L)
    (bind (_outhit _returnvalue_2) (Collision|LineTraceByChannel _worldlocation (+ _worldlocation (* _worlddirection 1e+04)) "TraceTypeQuery1" true 0 "None" false "(R=1.000000,G=0.000000,B=0.000000,A=1.000000)" "(R=0.000000,G=1.000000,B=0.000000,A=1.000000)" 1.0))
    (if _returnvalue_2
      (bind _asbp_whiteboard (Utilities|Casting|CastToBP_whiteboard_NOTTHIS (.HitActor (Collision|BreakHitResult _outhit))))
      (CallFunction|DrawonWhiteboard _asbp_whiteboard (.UV (Class|GameplayStatics|FindCollisionUV _outhit))))))

(event Input|MouseEvents|LeftMouseButton
  (params (Key :type Key%20Structure :default "None"))
  (:Pressed
    (Variables|Default|SetMousepressed%20L true))
  (:Released
    (Variables|Default|SetMousepressed%20L false)))

(fn ConstructionScript)