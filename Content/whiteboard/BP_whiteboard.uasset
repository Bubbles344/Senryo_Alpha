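; BP_whiteboard is a mouse-drawn whiteboard with symbol recognition, which moves itself to a "WB" actor matched by name number on BeginPlay.
; Held-click traces convert hit UVs into sharpie material draws on a render target.
; MouseTick samples screen points with stroke numbers into Push, marked as sending to JavaScript.
; Enter calls Rec and displays LastSymbol, Backspace clears everything; Push, Rec and ClearArr are empty here, and SymbolHandler only prints.
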(event Custom|DrawOnWhiteboard
  (params (locationtodraw :type Vector%202D%20Structure))
  (bind _sharpieinstance (Variables|Default|GetSharpieInstance))
  ;[1 1 1] SETUP
  (Rendering|Material|SetVectorParameterValue _sharpieinstance "drawLocation" (Math|Conversions|ToLinearColor(Vector) (Math|Conversions|ToVector(Vector2D) locationtodraw)) :!class /Script/Engine.MaterialInstanceDynamic)
  (Rendering|DrawMaterialtoRenderTarget "/Game/whiteboard/RT_WHITEBOARD.RT_WHITEBOARD" _sharpieinstance))

(event Custom|MouseTick
  ;[1 1 1] SEND POINTS TO JAVASCRIPT
  (if (Math|Boolean|ANDBoolean (== (Math|Integer|%(Integer) (Math|Conversions|ToInteger(Byte) (Utilities|GetFrameCount)) (Variables|Default|GetSampleRate)) 0) (Variables|Default|GetMousepressed%20L) (Utilities|String|Contains (Utilities|GetDisplayName (.HitActor (Collision|BreakHitResult (stale Input|AxisEvents|InputAxisMouseMove _outhit)))) (Utilities|String|GetSubstring (Utilities|GetDisplayName self) 9 2)))
    (bind _returnvalue (Class|WidgetLayoutLibrary|GetMousePositiononViewport))
    (Development|PrintString (Utilities|String|Append "X: " (Utilities|String|ToString(Integer) (Math|Float|Truncate (.x _returnvalue))) ", Y: " (Utilities|String|ToString(Integer) (Math|Float|Truncate (.y _returnvalue))) ", STROKE: " (Utilities|String|ToString(Integer) (Variables|Default|GetStroke)) ", OBJECT: " (Utilities|GetDisplayName self)))
    (CallFunction|Push (Math|Float|Truncate (.x _returnvalue)) (Math|Float|Truncate (.y _returnvalue)) (Variables|Default|GetStroke))))

(event Custom|Locate
  (bind _self self)
  (bind _actorarr (Variables|Default|GetActorArr))
  (bind _returnvalue (Utilities|Array|Length _actorarr))
  (bind _returnvalue_2 (Utilities|GetDisplayName _self))
  (bind _returnvalue_3 (Utilities|String|GetSubstring _returnvalue_2 9 2))
  (bind _returnvalue_4 (* _returnvalue 2))
  (bind _returnvalue_5 (Math|Conversions|ToInteger(Byte) _returnvalue_3))
  (bind _returnvalue_6 (+ _returnvalue_5 _returnvalue_4))
  (bind _returnvalue_7 (Utilities|String|ToString(Integer) _returnvalue_6))
  ;[1 1 1] LOCATE OWNER AND MOVE TO LOCATION
  (bind _outactors (Actor|GetAllActorsOfClass "/Script/Engine.Actor"))
  (bind _index (Utilities|FlowControl|ForLoopwithBreak 0 (- (Utilities|Array|Length _outactors) 1))
    (:LoopBody
      (if (Utilities|String|Contains (Utilities|GetDisplayName (Utilities|Array|Get(acopy) _outactors _index)) "WB")
        (Utilities|Array|Add (Variables|Default|GetActorArr) (Utilities|Array|Get(acopy) _outactors _index))))
    (:Completed
      (bind _index_2 (Utilities|FlowControl|ForLoopwithBreak 0 (- (Utilities|Array|Length (Variables|Default|GetActorArr)) 1))
        (:LoopBody
          (if (or (Utilities|String|Contains (Utilities|GetDisplayName (Utilities|Array|Get(acopy) (Variables|Default|GetActorArr) _index_2)) (Utilities|String|ToString(Integer) (/ (+ _returnvalue_5 1) 2)) false true) (Utilities|String|Contains (Utilities|GetDisplayName (Utilities|Array|Get(acopy) (Variables|Default|GetActorArr) _index_2)) _returnvalue_7 false true))
            (Development|PrintString (Utilities|String|Append "MOVING TO: " (Utilities|GetDisplayName (Utilities|Array|Get(acopy) (Variables|Default|GetActorArr) _index_2))))
            (Transformation|SetActorLocation (Transformation|GetActorLocation (Utilities|Array|Get(acopy) (Variables|Default|GetActorArr) _index_2)) false true)))
        (:Completed
          (Development|PrintString (Utilities|String|Append "NUMBER: " _returnvalue_3 ", OR: " _returnvalue_7)))))))

(event Custom|SymbolHandler
  (switch string (Variables|Default|GetlastSymbol)
    (:Default
      (Development|PrintString "SWITCH DEF"))
    (:X
      (Development|PrintString "SWITCH X"))
    (:T
      (Development|PrintString "SWITCH T"))
    (:H
      (Development|PrintString "SWITCH H"))
    (:n
      (Development|PrintString "SWITCH N"))))

(event EventBeginPlay
  ;[1 1 1] SETUP
  (CallFunction|Locate)
  (Input|EnableInput (Game|GetPlayerController 0))
  (bind _returnvalue (Rendering|Material|CreateDynamicMaterialInstance "/Game/whiteboard/M_sharpie.M_sharpie" "None" "None" :!class /Script/Engine.KismetMaterialLibrary))
  (Variables|Default|SetSharpieInstance _returnvalue)
  (Rendering|ClearRenderTarget2D "/Game/whiteboard/RT_WHITEBOARD.RT_WHITEBOARD"))

(event Input|AxisEvents|InputAxisMouseMove
  (params (AxisValue :type Float%20%28single-precision%29))
  (bind _returnvalue (Game|GetPlayerController 0))
  (bind (_worldlocation _worlddirection) (Game|Player|ConvertMouseLocationToWorldSpace _returnvalue))
  ;[1 1 1] LINE TRACE
  (CallFunction|MouseTick)
  (if (Variables|Default|GetMousepressed%20L)
    (bind (_outhit _returnvalue_2) (Collision|LineTraceByChannel _worldlocation (+ _worldlocation (* _worlddirection 1e+04)) "TraceTypeQuery1" true 0 "None" false "(R=1.000000,G=0.000000,B=0.000000,A=1.000000)" "(R=0.000000,G=1.000000,B=0.000000,A=1.000000)" 1.0))
    (if _returnvalue_2
      (bind _asbp_whiteboard (Utilities|Casting|CastToBP_whiteboard (.HitActor (Collision|BreakHitResult _outhit))))
      (CallFunction|DrawonWhiteboard _asbp_whiteboard (.UV (Class|GameplayStatics|FindCollisionUV _outhit))))))

(event Input|KeyboardEvents|Backspace
  (params (Key :type Key%20Structure :default "None"))
  (:Pressed
    (CallFunction|ClearArr)
    (Rendering|Components|TextRender|SetText (Variables|Default|GetTextRender) (Utilities|Text|ToText(String) ""))
    (Rendering|ClearRenderTarget2D "/Game/whiteboard/RT_WHITEBOARD.RT_WHITEBOARD")))

(event Input|MouseEvents|LeftMouseButton
  (params (Key :type Key%20Structure :default "None"))
  ;[1 1 1] SEND POINTS TO JAVASCRIPT
  (:Pressed
    (Variables|Default|SetMousepressed%20L true))
  (:Released
    (Variables|Default|SetMousepressed%20L false)
    (Math|Integer|IncrementInt (Variables|Default|GetStroke))))

(event Input|KeyboardEvents|Enter
  (params (Key :type Key%20Structure :default "None"))
  (bind _lastsymbol (Variables|Default|GetlastSymbol))
  (:Pressed
    (Variables|Default|SetStroke 1)
    (CallFunction|Rec)
    (CallFunction|SymbolHandler)
    (Development|PrintString (Utilities|String|Append "Symbol: " _lastsymbol))
    (Rendering|Components|TextRender|SetText (Variables|Default|GetTextRender) (Utilities|Text|ToText(String) _lastsymbol))))

(fn ConstructionScript)

(fn NewFunction
  (params (x :type Integer) (y :type Integer))
  (Development|PrintString "NOPE"))

(fn Push
  (params (x :type Integer) (y :type Integer) (stroke :type Integer)))

(fn Rec
  (return))

(fn ClearArr)