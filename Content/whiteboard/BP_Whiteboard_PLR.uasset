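; Player whiteboard actor for drawing symbols by mouse, shown where right-click hits a fixed plane and hidden after release.
; Left-drag line-traces to the hit UV and paints a sharpie material into a render target.
; Sampled screen points and stroke numbers feed Push, marked for JavaScript.
; Right release calls Rec, displays LastSymbol, then clears; Push, Rec and ClearArr are empty here, and SymbolHandler only casts for "+".
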(event Custom|DrawOnWhiteboard
  (params (locationtodraw :type Vector%202D%20Structure))
  (bind _sharpieinstance (Variables|Default|GetSharpieInstance))
  ;[1 1 1] SETUP
  (Rendering|Material|SetVectorParameterValue _sharpieinstance "drawLocation" (Math|Conversions|ToLinearColor(Vector) (Math|Conversions|ToVector(Vector2D) locationtodraw)) :!class /Script/Engine.MaterialInstanceDynamic)
  (Rendering|DrawMaterialtoRenderTarget "/Game/whiteboard/RT_WHITEBOARD_PLR.RT_WHITEBOARD_PLR" _sharpieinstance))

(event Custom|MouseTick
  ;[1 1 1] SEND POINTS TO JAVASCRIPT
  (if (Math|Boolean|ANDBoolean (== (Math|Integer|%(Integer) (Math|Conversions|ToInteger(Byte) (Utilities|GetFrameCount)) (Variables|Default|GetSampleRate)) 0) (Variables|Default|GetMousepressed%20L) (Utilities|String|Contains (Utilities|GetDisplayName (.HitActor (Collision|BreakHitResult (stale Input|AxisEvents|InputAxisMouseMove _outhit)))) (Utilities|String|GetSubstring (Utilities|GetDisplayName self) 9 2)) (Variables|Default|GetMousepressed%20R))
    (bind _returnvalue (Class|WidgetLayoutLibrary|GetMousePositiononViewport))
    (Development|PrintString (Utilities|String|Append "X: " (Utilities|String|ToString(Integer) (Math|Float|Truncate (.x _returnvalue))) ", Y: " (Utilities|String|ToString(Integer) (Math|Float|Truncate (.y _returnvalue))) ", STROKE: " (Utilities|String|ToString(Integer) (Variables|Default|GetStroke)) ", OBJECT: " (Utilities|GetDisplayName self)))
    (CallFunction|Push (Math|Float|Truncate (.x _returnvalue)) (Math|Float|Truncate (.y _returnvalue)) (Variables|Default|GetStroke))))

(event Custom|SymbolHandler
  (switch string (Variables|Default|GetlastSymbol)
    (:+
      (bind _returnvalue (Actor|GetActorOfClass "/Game/2DSideScrollerBP/Blueprints/2DSideScrollerCharacter.2DSideScrollerCharacter_C"))
      (Utilities|Casting|CastTo2DSideScrollerCharacter _returnvalue))))

(event EventBeginPlay
  ;[1 1 1] SETUP
  (Transformation|SetActorLocation "0, 0,-200.000000" false false)
  (Input|EnableInput (Game|GetPlayerController 0))
  (bind _returnvalue (Rendering|Material|CreateDynamicMaterialInstance "/Game/whiteboard/M_sharpie.M_sharpie" "None" "None" :!class /Script/Engine.KismetMaterialLibrary))
  (Variables|Default|SetSharpieInstance _returnvalue)
  (Rendering|ClearRenderTarget2D "/Game/whiteboard/RT_WHITEBOARD_PLR.RT_WHITEBOARD_PLR"))

(event Input|AxisEvents|InputAxisMouseMove
  (params (AxisValue :type Float%20%28single-precision%29))
  (bind _returnvalue (Game|GetPlayerController 0))
  (bind (_worldlocation _worlddirection) (Game|Player|ConvertMouseLocationToWorldSpace _returnvalue))
  ;[1 1 1] LINE TRACE
  (CallFunction|MouseTick)
  (if (Variables|Default|GetMousepressed%20L)
    (bind (_outhit _returnvalue_2) (Collision|LineTraceByChannel _worldlocation (+ _worldlocation (* _worlddirection 1e+04)) "TraceTypeQuery1" true 0 "None" false "(R=1.000000,G=0.000000,B=0.000000,A=1.000000)" "(R=0.000000,G=1.000000,B=0.000000,A=1.000000)" 1.0))
    (if _returnvalue_2
      (bind _asbp_whiteboard_plr (Utilities|Casting|CastToBP_Whiteboard_PLR (.HitActor (Collision|BreakHitResult _outhit))))
      (CallFunction|DrawonWhiteboard _asbp_whiteboard_plr (.UV (Class|GameplayStatics|FindCollisionUV _outhit))))))

(event Input|KeyboardEvents|Backspace
  (params (Key :type Key%20Structure :default "None"))
  (:Pressed
    (CallFunction|ClearArr)
    (Rendering|Components|TextRender|SetText (Variables|Default|GetTextRender) (Utilities|Text|ToText(String) ""))
    (Rendering|ClearRenderTarget2D "/Game/whiteboard/RT_WHITEBOARD_PLR.RT_WHITEBOARD_PLR")))

(event Input|MouseEvents|RightMouseButton
  (params (Key :type Key%20Structure :default "None"))
  (bind _returnvalue (Game|GetPlayerController 0))
  (bind _lastsymbol (Variables|Default|GetlastSymbol))
  (bind (_worldlocation _worlddirection) (Game|Player|ConvertMouseLocationToWorldSpace _returnvalue))
  (:Pressed
    (Variables|Default|SetMousepressed%20R true)
    (Transformation|SetActorLocation (.Intersection (Class|KismetMathLibrary|LinePlaneIntersectionOriginNormal _worldlocation (+ _worldlocation (* _worlddirection 1e+04)) "0,100.000000, 0" "0,-1.000000, 0")) false false))
  (:Released
    (Variables|Default|SetMousepressed%20R true)
    (CallFunction|Rec)
    (CallFunction|SymbolHandler)
    (Development|PrintString (Utilities|String|Append "Symbol: " _lastsymbol))
    (Rendering|Components|TextRender|SetText (Variables|Default|GetTextRender) (Utilities|Text|ToText(String) _lastsymbol))
    (Variables|Default|SetStroke 1)
    (Utilities|FlowControl|Delay 1.0)
    (Transformation|SetActorLocation "0, 0,-200.000000" false false)
    (CallFunction|ClearArr)
    (Rendering|Components|TextRender|SetText (Variables|Default|GetTextRender) (Utilities|Text|ToText(String) ""))
    (Rendering|ClearRenderTarget2D "/Game/whiteboard/RT_WHITEBOARD_PLR.RT_WHITEBOARD_PLR")))

(event Input|MouseEvents|LeftMouseButton
  (params (Key :type Key%20Structure :default "None"))
  ;[1 1 1] SEND POINTS TO JAVASCRIPT
  (:Pressed
    (Variables|Default|SetMousepressed%20L true))
  (:Released
    (Variables|Default|SetMousepressed%20L false)
    (Math|Integer|IncrementInt (Variables|Default|GetStroke))))

(fn ConstructionScript)

(fn NewFunction
  (params (x :type Integer) (y :type Integer))
  (Development|PrintString "NOPE"))

(fn Push
  (params (x :type Integer) (y :type Integer) (stroke :type Integer)))

(fn Rec
  (return))

(fn ClearArr)